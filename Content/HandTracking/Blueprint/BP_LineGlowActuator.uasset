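; BP_LineGlowActuator pulses the hologram line glow outward from its origin and back.
; GlowLinesInAndOut plays or reverses a timeline based on GlowIn, lerping the LineGlowFromOrigin scalar in the MPC_GlobalHologram material parameter collection.
; On finish it flips GlowIn and sets a timer: a short hold before reversing, a random multi-second pause before playing forward.
; The graph contains no BeginPlay or other trigger for the first pulse.
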(event `GlowLinesInAndOut`
  (if (`self.GlowIn?`)
    (bind (_direction _alpha) (`Timeline|GlowTimeLine` :!label _label)
      (:`Update`
        (`KismetMaterialLibrary.SetScalarParameterValue` "/Game/HandTracking/Material/ParamCollection/MPC_GlobalHologram.MPC_GlobalHologram" "LineGlowFromOrigin" (`KismetMathLibrary.Lerp` 0.0 1500.0 _alpha)))
      (:`Finished`
        (set `self.GlowIn?` (not (`self.GlowIn?`)))
        (`KismetSystemLibrary.K2_SetTimerDelegate` (`|CreateDelegate` :!event `GlowLinesInAndOut`) (`KismetMathLibrary.SelectFloat` (`KismetMathLibrary.RandomFloatInRange` 5.0 10.0) 0.5 (`self.GlowIn?`)))))
    (else
      (goto _label :!via `Reverse`))))

(fn `UserConstructionScript`)