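; TaskHolder is an actor that runs a hand-tracking test task, wrapping a Task object and presenting each objective with hologram effects.
; BeginTesting starts the task, plays intro reveal timelines, then begins the first objective and spawns a push button that completes objectives.
; Task events drive timelines that animate MPC_GlobalHologram parameters to show objective actors, glow their lines when ready, and hide them before cleanup and advancing.
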(event `self.ReceiveBeginPlay`
  (add `HTTask.OnTaskObjectiveCompleted` (`self.Task`) (delegate `OnTaskObjectiveCompleted_Event`))
  (`KismetMaterialLibrary.SetScalarParameterValue` "/Game/HandTracking/Material/ParamCollection/MPC_GlobalHologram.MPC_GlobalHologram" "TaskActorZVisibility")
  (`KismetMaterialLibrary.SetScalarParameterValue` "/Game/HandTracking/Material/ParamCollection/MPC_GlobalHologram.MPC_GlobalHologram" "GlobalZVisibility")
  (`KismetMaterialLibrary.SetScalarParameterValue` "/Game/HandTracking/Material/ParamCollection/MPC_GlobalHologram.MPC_GlobalHologram" "IntroDistanceFromOrigin")
  (add `HTTask.OnObjectiveStarted` (`self.Task`) (`|CreateDelegate` :!event `OnObjectiveStarted`)))

(event `OnTaskObjectiveCompleted_Event`
  (params (Objective :type "HTTaskObjective Object Reference") (ObjectiveIndex :type Integer))
  (`self.OnObjectiveReadyToBeCompleted` false)
  (bind (_direction _alpha) (`Timeline|HideObjectiveActorsTimeline` :!via `PlayFromStart`)
    (:`Update`
      (`KismetMaterialLibrary.SetScalarParameterValue` "/Game/HandTracking/Material/ParamCollection/MPC_GlobalHologram.MPC_GlobalHologram" "TaskActorZVisibility" (`KismetMathLibrary.Lerp` 150.0 0.0 _alpha)))
    (:`Finished`
      (`HTTaskObjective.CleanUp` Objective)
      (`self.BeginNextObjective`))))

(event `BeginTesting`
  (params (Configuration :type String))
  (`|ExecutionSequence`
    (:`then_0`
      (`HTTask.StartTask` (`self.Task`) null Configuration)
      (add `HTTask.OnObjectiveReadyToBeCompleted` (`self.Task`) (`|CreateDelegate` :!event `OnObjectiveReadyToBeCompleted`)))
    (:`then_1`
      (bind (_direction _alpha) (`Timeline|StartTimeline`)
        (:`Update`
          (`KismetMaterialLibrary.SetScalarParameterValue` "/Game/HandTracking/Material/ParamCollection/MPC_GlobalHologram.MPC_GlobalHologram" "IntroDistanceFromOrigin" (`KismetMathLibrary.Lerp` 0.0 1500.0 _alpha)))
        (:`Finished`
          (bind (_direction_2 _alpha_2) (`Timeline|GlobalZVisibility`)
            (:`Update`
              (`KismetMaterialLibrary.SetScalarParameterValue` "/Game/HandTracking/Material/ParamCollection/MPC_GlobalHologram.MPC_GlobalHologram" "GlobalZVisibility" (`KismetMathLibrary.Lerp` 0.0 200.0 _alpha_2)))
            (:`Finished`
              (`self.BeginNextObjective`)
              (bind _returnvalue (`GameplayStatics.GetActorOfClass` "/Game/HandTracking/Blueprint/BP_LineGlowActuator.BP_LineGlowActuator_C"))
              (`/Game/HandTracking/Blueprint/BP_LineGlowActuator.GlowLinesInAndOut` _returnvalue)
              (bind _returnvalue_2 (`|SpawnActorFromClass` :`Class` "/Game/HandTracking/Blueprint/BP_PushButton_FinishObjective.BP_PushButton_FinishObjective_C" :`SpawnTransform` (`KismetMathLibrary.MakeTransform` (25.0 55.0 70.0)) :`CollisionHandlingOverride` "Undefined" :`TransformScaleMethod` "MultiplyWithRoot" :`ButtonMesh` "/Game/HandTracking/Meshes/Button.Button" :`AttachTo` null :`Instigator` null))
              (set `/OculusHandTools/Button/PushButtonBaseBP.ActorsToActionOnPress` (`|MakeArray` self :!type "Actor Object Reference") _returnvalue_2))))))))

(event `/OculusHandTools/Button/IsButtonableInterface.ButtonAction`
  (params (Action :type Name))
  (if (== Action "ProceedObjective")
    (`HTTask.CompleteCurrentObjective` (`self.Task`))))

(event `BeginNextObjective`
  (`HTTask.BeginNextObjective` (`self.Task`) null))

(event `OnObjectiveStarted`
  (params (Objective :type "HTTaskObjective Object Reference") (ObjectiveIndex :type Integer))
  (bind (_direction _alpha) (`Timeline|ShowObjectiveActorsTimeline` :!via `PlayFromStart`)
    (:`Update`
      (`KismetMaterialLibrary.SetScalarParameterValue` "/Game/HandTracking/Material/ParamCollection/MPC_GlobalHologram.MPC_GlobalHologram" "TaskActorZVisibility" (`KismetMathLibrary.Lerp` 0.0 200.0 _alpha)))))

(event `OnObjectiveReadyToBeCompleted`
  (params (bReady :type Boolean))
  (if bReady
    (bind (_direction _alpha) (`Timeline|LineGlowObjectiveTimeline` :!label _label)
      (:`Update`
        (`KismetMaterialLibrary.SetScalarParameterValue` "/Game/HandTracking/Material/ParamCollection/MPC_GlobalHologram.MPC_GlobalHologram" "FadeObjectiveActorLines" (`KismetMathLibrary.Lerp` 0.0 150.0 _alpha))))
    (else
      (goto _label :!via `Reverse`))))

(fn `UserConstructionScript`)