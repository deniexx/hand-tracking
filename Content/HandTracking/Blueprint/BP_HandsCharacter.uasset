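; VR player character for a test comparing motion controllers, hand tracking and haptic hand tracking.
; Enhanced Input actions start each test mode through the level's TaskHolder, reload L_Basic or recenter the headset.
; Left and right grab components pick up objects at the controller transforms, notify them on grab and release, and play controller haptics on pickup.
; Grabbing an object held by the other hand releases it there, handing it over.
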(event `EnhancedInput|/Game/HandTracking/Input/IA_Restart`
  (params (ActionValue :type Boolean) (ElapsedSeconds :type "Float (double-precision)") (TriggeredSeconds :type "Float (double-precision)") (InputAction :type "InputAction Object Reference" :default "/Game/HandTracking/Input/IA_Restart.IA_Restart"))
  (:`Started`
    (`GameplayStatics.OpenLevelBySoftObjectPtr` "/Game/L_Basic.L_Basic")))

(event `EnhancedInput|/Game/HandTracking/Input/IA_BeginController`
  (params (ActionValue :type Boolean) (ElapsedSeconds :type "Float (double-precision)") (TriggeredSeconds :type "Float (double-precision)") (InputAction :type "InputAction Object Reference" :default "/Game/HandTracking/Input/IA_BeginController.IA_BeginController"))
  (:`Started`
    (bind _returnvalue (`GameplayStatics.GetActorOfClass` "/Game/HandTracking/Blueprint/TaskHolder.TaskHolder_C"))
    (`/Game/HandTracking/Blueprint/TaskHolder.BeginTesting` _returnvalue "MotionControllers")))

(event `EnhancedInput|/Game/HandTracking/Input/IA_BeginHandTracking`
  (params (ActionValue :type Boolean) (ElapsedSeconds :type "Float (double-precision)") (TriggeredSeconds :type "Float (double-precision)") (InputAction :type "InputAction Object Reference" :default "/Game/HandTracking/Input/IA_BeginHandTracking.IA_BeginHandTracking"))
  (:`Started`
    (bind _returnvalue (`GameplayStatics.GetActorOfClass` "/Game/HandTracking/Blueprint/TaskHolder.TaskHolder_C"))
    (`/Game/HandTracking/Blueprint/TaskHolder.BeginTesting` _returnvalue "HandTracking")))

(event `EnhancedInput|/Game/HandTracking/Input/IA_BeginHapticHandTracking`
  (params (ActionValue :type Boolean) (ElapsedSeconds :type "Float (double-precision)") (TriggeredSeconds :type "Float (double-precision)") (InputAction :type "InputAction Object Reference" :default "/Game/HandTracking/Input/IA_BeginHapticHandTracking.IA_BeginHapticHandTracking"))
  (:`Started`
    (bind _returnvalue (`GameplayStatics.GetActorOfClass` "/Game/HandTracking/Blueprint/TaskHolder.TaskHolder_C"))
    (`/Game/HandTracking/Blueprint/TaskHolder.BeginTesting` _returnvalue "HapticHandTracking")))

(event `self.ReceiveBeginPlay`
  (`parent.ReceiveBeginPlay`)
  (`EnhancedInputSubsystemInterface.AddMappingContext` (pcsubsystem `EnhancedInputLocalPlayerSubsystem` (`GameplayStatics.GetPlayerController` 0)) "/Game/HandTracking/Input/IMC_Default.IMC_Default" 0 (struct)))

(event `EnhancedInput|/Game/HandTracking/Input/IA_GrabLeft`
  (params (ActionValue :type Boolean) (ElapsedSeconds :type "Float (double-precision)") (TriggeredSeconds :type "Float (double-precision)") (InputAction :type "InputAction Object Reference" :default "/Game/HandTracking/Input/IA_GrabLeft.IA_GrabLeft"))
  ;[1 1 1] Grabbing
  (:`Started`
    (bind _returnvalue (`HandGrabbingComponent.TryGrab` (`self.LeftGrabbing`) (`SceneComponent.K2_GetComponentToWorld` (`self.MotionControllerLeft`))))
    (`/Engine/EditorBlueprintResources/StandardMacros.IsValid` _returnvalue
      (:`Is Valid`
        (bind _output_get (set `self.LeftGrabObject` _returnvalue))
        (`Interactable.Interaction2` _output_get)
        (`OculusXRInputFunctionLibrary.PlayCurveHapticEffect` "/Game/HandTracking/Haptics/HF_GrabDrop.HF_GrabDrop" "Left")
        (if (== (`self.LeftGrabObject`) (`self.RightGrabObject`))
          (bind _returnvalue_2 (`HandGrabbingComponent.TryRelease` (`self.RightGrabbing`) false))
          (`/Engine/EditorBlueprintResources/StandardMacros.IsValid` _returnvalue_2
            (:`Is Valid`
              (`Interactable.Interaction3` _returnvalue_2))
            (:`Is Not Valid`
              _))
          (set `self.RightGrabObject` null)))))
  (:`Completed`
    (bind _returnvalue_3 (`HandGrabbingComponent.TryRelease` (`self.LeftGrabbing`) false))
    (`/Engine/EditorBlueprintResources/StandardMacros.IsValid` _returnvalue_3
      (:`Is Valid`
        (`Interactable.Interaction3` _returnvalue_3))
      (:`Is Not Valid`
        _))
    (set `self.LeftGrabObject` null)))

(event `EnhancedInput|/Game/HandTracking/Input/IA_GrabRight`
  (params (ActionValue :type Boolean) (ElapsedSeconds :type "Float (double-precision)") (TriggeredSeconds :type "Float (double-precision)") (InputAction :type "InputAction Object Reference" :default "/Game/HandTracking/Input/IA_GrabRight.IA_GrabRight"))
  ;[1 1 1] Grabbing
  (:`Started`
    (bind _returnvalue (`HandGrabbingComponent.TryGrab` (`self.RightGrabbing`) (`SceneComponent.K2_GetComponentToWorld` (`self.MotionControllerRight`))))
    (`/Engine/EditorBlueprintResources/StandardMacros.IsValid` _returnvalue
      (:`Is Valid`
        (bind _output_get (set `self.RightGrabObject` _returnvalue))
        (`Interactable.Interaction2` _output_get)
        (`OculusXRInputFunctionLibrary.PlayCurveHapticEffect` "/Game/HandTracking/Haptics/HF_GrabDrop.HF_GrabDrop" "Right")
        (if (== (`self.LeftGrabObject`) (`self.RightGrabObject`))
          (bind _returnvalue_2 (`HandGrabbingComponent.TryRelease` (`self.LeftGrabbing`) false))
          (`/Engine/EditorBlueprintResources/StandardMacros.IsValid` _returnvalue_2
            (:`Is Valid`
              (`Interactable.Interaction3` _returnvalue_2))
            (:`Is Not Valid`
              _))
          (set `self.LeftGrabObject` null)))))
  (:`Completed`
    (bind _returnvalue_3 (`HandGrabbingComponent.TryRelease` (`self.RightGrabbing`) false))
    (`/Engine/EditorBlueprintResources/StandardMacros.IsValid` _returnvalue_3
      (:`Is Valid`
        (`Interactable.Interaction3` _returnvalue_3))
      (:`Is Not Valid`
        _))
    (set `self.RightGrabObject` null)))

(event `EnhancedInput|/Game/HandTracking/Input/IA_Recenter`
  (params (ActionValue :type Boolean) (ElapsedSeconds :type "Float (double-precision)") (TriggeredSeconds :type "Float (double-precision)") (InputAction :type "InputAction Object Reference" :default "/Game/HandTracking/Input/IA_Recenter.IA_Recenter"))
  (:`Completed`
    (`HeadMountedDisplayFunctionLibrary.ResetOrientationAndPosition` 0.0)))

(fn `UserConstructionScript`
  (`parent.UserConstructionScript`))