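; BP_Button is a push button for the hand-tracking minigames that reports its button number when touched by the player's hands character.
; An overlap from BP_HandsCharacter on its StaticMesh fires OnButtonPressed and plays the PushButton timeline, ignoring new overlaps while that timeline runs.
; The timeline lerps the whole actor between its starting location and a point slightly offset along world X, both cached at BeginPlay.
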(event `self.ReceiveBeginPlay`
  (bind _output_get (set `self.StartPos` (`self.K2_GetActorLocation`)))
  (set `self.TargetPos` (`KismetMathLibrary.MakeVector` (+ (.x _output_get) 0.5) (.y _output_get) (.z _output_get))))

(event `self.StaticMesh.OnComponentBeginOverlap`
  (params (OverlappedComponent :type "PrimitiveComponent Object Reference") (OtherActor :type "Actor Object Reference") (OtherComp :type "PrimitiveComponent Object Reference") (OtherBodyIndex :type Integer) (bFromSweep :type Boolean) (SweepResult :type "HitResult Structure (by ref)"))
  (if (not (`TimelineComponent.IsPlaying` (`self.PushButton`)))
    (cast `/Game/HandTracking/Blueprint/BP_HandsCharacter` OtherActor)
    (`self.OnButtonPressed` (`self.ButtonNumber`))
    (bind (_direction _alpha) (`Timeline|PushButton` :!via `PlayFromStart`)
      (:`Update`
        (`self.K2_SetActorLocation` (`KismetMathLibrary.VLerp` (`self.StartPos`) (`self.TargetPos`) _alpha))))))

(fn `UserConstructionScript`)