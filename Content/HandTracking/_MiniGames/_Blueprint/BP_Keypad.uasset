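; Keypad for a hand-tracking mini-game where the player enters a random four-digit code conveyed through hand feedback.
; ButtonAction generates the code, runs the clear handler, then signals each digit through a delayed, self-calling event.
; Button presses fill a capped entry array and the WBP_Buttons display.
; The clear button doubles as submit: a match loads L_MiniGames after a success sound, otherwise it plays a failure sound and wipes the entry.
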(event `self.ReceiveBeginPlay`
  (`HTBlueprintFunctionLibrary.ToggleHandFeedback` true)
  (for _array_element (`self.Buttons`)
    (add `/Game/HandTracking/_MiniGames/_Blueprint/Buttons/BP_Button.OnButtonPressed` _array_element (`|CreateDelegate` :!event `OnButtonPressedEvent`)))
  (add `/Game/HandTracking/_MiniGames/_Blueprint/Buttons/BP_Button.OnButtonPressed` (`self.ClearButton`) (delegate `OnClearButtonPressed`)))

(event `OnClearButtonPressed`
  (params (ButtonNumber :type Integer))
  (bind _result (`self.EvaluateCorrectCode`))
  (if _result
    (`GameplayStatics.PlaySound2D` "/Engine/EditorSounds/Notifications/CompileSuccess_Cue.CompileSuccess_Cue" 1.0 1.0 0.0 null null)
    (`KismetSystemLibrary.Delay` 2.0)
    (`GameplayStatics.OpenLevelBySoftObjectPtr` "/Game/HandTracking/Maps/L_MiniGames.L_MiniGames")
    (else
      (`GameplayStatics.PlaySound2D` "/Engine/EditorSounds/Notifications/CompileFailed_Cue.CompileFailed_Cue" 1.0 1.0 0.0 null null)
      (`KismetArrayLibrary.Array_Clear` (`self.PressedNumbers`))
      (bind _aswbp_buttons (cast `/Game/HandTracking/_MiniGames/_Blueprint/WBP_Buttons` (`WidgetComponent.GetWidget` (`self.Widget`))))
      (`/Game/HandTracking/_MiniGames/_Blueprint/WBP_Buttons.ClearCode` _aswbp_buttons))))

(event `/OculusHandTools/Button/IsButtonableInterface.ButtonAction`
  (params (Action :type Name))
  (set `self.Iteration` 0)
  (bind _outnumbers (`HTBlueprintFunctionLibrary.GenerateRandomNumbersArray` 4))
  (set `self.TargetNumbers` _outnumbers)
  (`self.OnClearButtonPressed` 0)
  (`self.RecursivelyApplyFeedback`))

(event `RecursivelyApplyFeedback`
  (if (> (`KismetArrayLibrary.Array_Length` (`self.TargetNumbers`)) (`self.Iteration`))
    (`HTBlueprintFunctionLibrary.SendFeedbackBasedOnArray` (`|GetArrayItem` (`self.TargetNumbers`) (`self.Iteration`)))
    (`KismetSystemLibrary.Delay` 2.0)
    (`/Engine/EditorBlueprintResources/StandardMacros.IncrementInt` (`self.Iteration`)
      (:`  `
        (`self.RecursivelyApplyFeedback`)))))

(fn `EvaluateCorrectCode`
  (returns (Result :type Boolean))
  (if (== (`KismetArrayLibrary.Array_Length` (`self.PressedNumbers`)) (`KismetArrayLibrary.Array_Length` (`self.TargetNumbers`)))
    (for (_array_element _array_index) (`self.TargetNumbers`)
      (if (not (== _array_element (`|GetArrayItem` (`self.PressedNumbers`) _array_index)))
        (return false)))
    (return true)
    (else
      (return false))))

(fn `OnButtonPressedEvent`
  (params (ButtonNumber :type Integer))
  (if (not (== (`KismetArrayLibrary.Array_Length` (`self.PressedNumbers`)) (`KismetArrayLibrary.Array_Length` (`self.TargetNumbers`))))
    (`KismetArrayLibrary.Array_Add` (`self.PressedNumbers`) (`local.ButtonNumber`))
    (bind _aswbp_buttons (cast `/Game/HandTracking/_MiniGames/_Blueprint/WBP_Buttons` (`WidgetComponent.GetWidget` (`self.Widget`))))
    (`/Game/HandTracking/_MiniGames/_Blueprint/WBP_Buttons.AddCodeDigit` _aswbp_buttons (`local.ButtonNumber`))))

(fn `UserConstructionScript`)